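; BP_FPS_PlayerController is a first-person player controller that turns Enhanced Input actions into character movement and camera look.
; On possess it caches the pawn as BP_FPS_Character, and on BeginPlay it adds the IMC_BaseControls mapping context.
; IA_Move forwards its value to the character's BaseMovement.
; IA_LookAround drives yaw and inverted pitch, with Sensitivity scaling only pitch because the yaw multiply is left unconnected.
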(event `self.ReceivePossess`
  (params (PossessedPawn :type "Pawn Object Reference"))
  (bind _asbp_fps_character (cast `/Game/Blueprints/GameSettings/BP_FPS_Character` PossessedPawn))
  (set `self.MainCharacter` _asbp_fps_character))

(event `self.ReceiveBeginPlay`
  (`EnhancedInputSubsystemInterface.AddMappingContext` (subsystem `EnhancedInputLocalPlayerSubsystem`) "/Game/Inputs/IMC_BaseControls.IMC_BaseControls" 0 (struct)))

(event `EnhancedInput|/Game/Inputs/IA_Move`
  (params (ActionValue :type "Vector2D Structure") (ElapsedSeconds :type "Float (double-precision)") (TriggeredSeconds :type "Float (double-precision)") (InputAction :type "InputAction Object Reference" :default "/Game/Inputs/IA_Move.IA_Move"))
  (:`Triggered`
    (`/Game/Blueprints/GameSettings/BP_FPS_Character.Base Movement` (`self.MainCharacter`) ActionValue)))

(event `EnhancedInput|/Game/Inputs/IA_LookAround`
  (params (ActionValue :type "Vector2D Structure") (ElapsedSeconds :type "Float (double-precision)") (TriggeredSeconds :type "Float (double-precision)") (InputAction :type "InputAction Object Reference" :default "/Game/Inputs/IA_LookAround.IA_LookAround"))
  (:`Triggered`
    (`self.AddYawInput` ActionValue_X)
    (`self.AddPitchInput` (* (* ActionValue_Y (`self.Sensitivity`)) -1.0))))

(fn `UserConstructionScript`)